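; Conveyor belt that moves actors overlapping its Box along the Arrow's forward vector at a set Speed.
; Auto-activation or a Box overlap starts it, and it stops when its tracked actor list empties on end overlap.
; A looping Transport timer, set to the frame delta at activation, gathers and offsets actors without sweeping.
; A dynamic material's Speed_X parameter, derived from CurrentSpeed, is updated on activation changes.
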(event OnComponentBeginOverlap(Box)
  (params (OverlappedComponent :type Primitive%20Component%20Object%20Reference) (OtherActor :type Actor%20Object%20Reference) (OtherComp :type Primitive%20Component%20Object%20Reference) (OtherBodyIndex :type Integer) (bFromSweep :type Boolean) (SweepResult :type Hit%20Result%20Structure%20%28by%20ref%29))
  (CallFunction|DispatcherActivateEvent true))

(event OnComponentEndOverlap(Box)
  (params (OverlappedComponent :type Primitive%20Component%20Object%20Reference) (OtherActor :type Actor%20Object%20Reference) (OtherComp :type Primitive%20Component%20Object%20Reference) (OtherBodyIndex :type Integer))
  ;[1 1 1] end overlap
  (Utilities|Array|RemoveItem (Variables|Default|GetArrayOfActors) OtherActor)
  (if (<= (Utilities|Array|Length (Variables|Default|GetArrayOfActors)) 0)
    (CallFunction|DispatcherActivateEvent false)))

(event Custom|Dispatcher_Activate_Event
  (params (On/off :type Boolean))
  (if On/off
    (bind _output_get (Variables|Default|SetCurrentSpeed (Math|Interpolation|FInterpTo 0.0 (Variables|Settings|GetSpeed) (Utilities|Time|GetWorldDeltaSeconds) 3.0)))
    (Rendering|Material|SetScalarParameterValue (Variables|Default|Getmaterial) "Speed_X" (* (/ _output_get 1e+02) -1.0) :!class /Script/Engine.MaterialInstanceDynamic)
    (Utilities|Time|SetTimerbyFunctionName 0 "Transport" (Utilities|Time|GetWorldDeltaSeconds) true)
    (else
      (bind _output_get_2 (Variables|Default|SetCurrentSpeed 0.0))
      (Rendering|Material|SetScalarParameterValue (Variables|Default|Getmaterial) "Speed_X" _output_get_2 :!class /Script/Engine.MaterialInstanceDynamic)
      (Utilities|Time|ClearTimerbyFunctionName 0 "Transport"))))

(event EventBeginPlay
  (if (Variables|Settings|GetAutoActivate?)
    (CallFunction|DispatcherActivateEvent true)))

(fn ConstructionScript
  (bind _returnvalue (Rendering|Material|CreateDynamicMaterialInstance (Variables|Default|GetStaticMesh) 0 0 "None" :!class /Script/Engine.PrimitiveComponent))
  (Variables|Default|Setmaterial _returnvalue)
  (Rendering|Material|SetMaterial (Variables|Default|GetStaticMesh) 0 (Variables|Default|Getmaterial))
  (Rendering|Material|SetScalarParameterValue (Variables|Default|Getmaterial) "Speed_X" (* (/ (Variables|Default|GetCurrentSpeed) 1e+02) -1.0) :!class /Script/Engine.MaterialInstanceDynamic))

(fn Transport
  (Variables|Default|SetCurrentSpeed (Variables|Settings|GetSpeed))
  (for _array_element (Collision|GetOverlappingActors (Variables|Default|GetBox) 0 :!class /Script/Engine.PrimitiveComponent)
    (if (!= _array_element self)
      (Utilities|Array|AddUnique (Variables|Default|GetArrayOfActors) _array_element)))
  (for _array_element_2 (Variables|Default|GetArrayOfActors)
    (Transformation|AddActorWorldOffset _array_element_2 (* (Math|Vector|GetForwardVector (Variables|Default|GetArrow)) (* (Utilities|Time|GetWorldDeltaSeconds) (Variables|Default|GetCurrentSpeed))))))